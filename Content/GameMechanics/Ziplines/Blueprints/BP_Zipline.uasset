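; BP_Zipline is a placeable zipline that offers overlapping actors a ride in either direction between its two ends.
; The construction script and BeginPlay run InitCable, which moves the cable to StartTop and attaches its end to the Scene component.
; Each end's collider sends SetZiplineMessage to the overlapping actor with start and end positions ordered from that side, then disables it on exit.
; The actor itself performs no movement.
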(event `self.ReceiveBeginPlay`
  (`self.InitCable`))

(event `self.StartCollider.OnComponentBeginOverlap`
  (params (OverlappedComponent :type "PrimitiveComponent Object Reference") (OtherActor :type "Actor Object Reference") (OtherComp :type "PrimitiveComponent Object Reference") (OtherBodyIndex :type Integer) (bFromSweep :type Boolean) (SweepResult :type "HitResult Structure (by ref)"))
  (message `/Game/GameMechanics/Ziplines/Blueprints/BPI_ZiplineRider.SetZipline` OtherActor true (`SceneComponent.K2_GetComponentLocation` (`self.StartTop`)) (`SceneComponent.K2_GetComponentLocation` (`self.Scene`))))

(event `self.StartCollider.OnComponentEndOverlap`
  (params (OverlappedComponent :type "PrimitiveComponent Object Reference") (OtherActor :type "Actor Object Reference") (OtherComp :type "PrimitiveComponent Object Reference") (OtherBodyIndex :type Integer))
  (message `/Game/GameMechanics/Ziplines/Blueprints/BPI_ZiplineRider.SetZipline` OtherActor false (0.0 0.0 0.0) (0.0 0.0 0.0))
  (`KismetSystemLibrary.PrintString` "eNDED START"))

(event `self.EndCollider.OnComponentBeginOverlap`
  (params (OverlappedComponent :type "PrimitiveComponent Object Reference") (OtherActor :type "Actor Object Reference") (OtherComp :type "PrimitiveComponent Object Reference") (OtherBodyIndex :type Integer) (bFromSweep :type Boolean) (SweepResult :type "HitResult Structure (by ref)"))
  (message `/Game/GameMechanics/Ziplines/Blueprints/BPI_ZiplineRider.SetZipline` OtherActor true (`SceneComponent.K2_GetComponentLocation` (`self.Scene`)) (`SceneComponent.K2_GetComponentLocation` (`self.StartTop`))))

(event `self.EndCollider.OnComponentEndOverlap`
  (params (OverlappedComponent :type "PrimitiveComponent Object Reference") (OtherActor :type "Actor Object Reference") (OtherComp :type "PrimitiveComponent Object Reference") (OtherBodyIndex :type Integer))
  (message `/Game/GameMechanics/Ziplines/Blueprints/BPI_ZiplineRider.SetZipline` OtherActor false (0.0 0.0 0.0) (0.0 0.0 0.0)))

(fn `UserConstructionScript`
  (`self.InitCable`))