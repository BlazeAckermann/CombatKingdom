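; BP_Item is an item Blueprint that shows a screen-space interaction prompt while a player is in interaction range.
; Entering range creates an interaction widget at runtime, owned by that player's controller, and attaches it in a new widget component; exiting destroys the component.
; GetInteractionText and GetInteractionTextAttach supply the prompt's text and attach point, defaulting to "Interact" and the root component.
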(event `/Game/GameMechanics/InteractionInterface/InteractionInterface.OnInteractionRangeEntered`
  (params (Player :type "/Game/AnimStarterPack/Ue4ASP_Character Object Reference"))
  (`self.InteractionWidgetComponent`
    (:`then`)
    (:`else`
      (bind _returnvalue (`|CreateWidget` "/Game/GameMechanics/InteractionInterface/InteractionWidget.InteractionWidget_C" (cast `PlayerController` (`Pawn.GetController` Player) :!pure true) (`self.GetInteractionText`)))
      (bind _returnvalue_2 (`AddComponent|NODE_AddWidgetComponent-0`))
      (bind _output_get (set `self.InteractionWidgetComponent` _returnvalue_2))
      (`WidgetComponent.SetWidget` _output_get _returnvalue)
      (`WidgetComponent.SetWidgetSpace` _output_get "Screen")
      (`WidgetComponent.SetDrawAtDesiredSize` _output_get true)
      (`PrimitiveComponent.SetCollisionEnabled` _output_get "NoCollision")
      (`SceneComponent.K2_AttachToComponent` _output_get (`self.GetInteractionTextAttach`) "None" "SnapToTarget" "SnapToTarget" "SnapToTarget" true))))

(event `/Game/GameMechanics/InteractionInterface/InteractionInterface.OnInteractionRangeExit`
  (bind _interactionwidgetcomponent (`self.InteractionWidgetComponent`)
    (:`then`
      (`ActorComponent.K2_DestroyComponent` _interactionwidgetcomponent))
    (:`else`)))

(fn `GetInteractionText`
  (returns (Text :type Text))
  (return "Interact"))

(fn `GetInteractionTextAttach`
  (returns (AttachComponent :type "SceneComponent Object Reference"))
  (return (`self.DefaultSceneRoot`)))

(fn `UserConstructionScript`)